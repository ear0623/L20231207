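; Pressure-plate button actor that plays a burst and logo animation when a BP_ThirdPersonCharacter steps on it.
; Box overlaps call ButtonPressed and ButtonReleased only on authority.
; Pressing lowers the button, attaches a particle burst to UELogo and runs a timeline that yaws Scene and moves the logo vertically.
; Release sets the same lowered offset as pressing, so the button does not rise.
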(event OnComponentBeginOverlap(Box)
  (params (OverlappedComponent :type Primitive%20Component%20Object%20Reference) (OtherActor :type Actor%20Object%20Reference) (OtherComp :type Primitive%20Component%20Object%20Reference) (OtherBodyIndex :type Integer) (bFromSweep :type Boolean) (SweepResult :type Hit%20Result%20Structure%20%28by%20ref%29))
  (Utilities|Casting|CastToBP_ThirdPersonCharacter OtherActor)
  (Networking|SwitchHasAuthority
    (:Authority
      (CallFunction|ButtonPressed))))

(event OnComponentEndOverlap(Box)
  (params (OverlappedComponent :type Primitive%20Component%20Object%20Reference) (OtherActor :type Actor%20Object%20Reference) (OtherComp :type Primitive%20Component%20Object%20Reference) (OtherBodyIndex :type Integer))
  (Utilities|Casting|CastToBP_ThirdPersonCharacter OtherActor)
  (Networking|SwitchHasAuthority
    (:Authority
      (CallFunction|ButtonReleased))))

(event Custom|ButtonReleased
  (Transformation|SetRelativeLocation (Variables|Default|GetButton) "0.000000,0.000000,-10.000000" false false))

(event Custom|ButtonPressed
  (Transformation|SetRelativeLocation (Variables|Default|GetButton) "0.000000,0.000000,-10.000000" false false)
  (Effects|SpawnEmitterAttached "/Game/ExampleContent/NetworkFeatures/Effects/P_Particle_Burst.P_Particle_Burst" (Variables|Default|GetUELogo) "None" "0.000000,15.000000,0.000000")
  (bind (_direction _rotation _height) (Timeline|Timeline PlayFromStart)
    (:Update
      (Transformation|SetRelativeRotation (Variables|Default|GetScene) (Math|Rotator|MakeRotator 0.0 0.0 _rotation) false false)
      (Transformation|SetRelativeLocation (Variables|Default|GetUELogo) (Math|Vector|Lerp(Vector) "0.000000,-15.000000,0.000000" "0.000000,-15.000000,50.000000" _height) false false))))

(event EventBeginPlay)

(event Collision|EventActorBeginOverlap
  (params (OtherActor :type Actor%20Object%20Reference)))

(event EventTick
  (params (DeltaSeconds :type Float%20%28single-precision%29)))

(fn ConstructionScript)