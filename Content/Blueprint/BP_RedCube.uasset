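; BP_RedCube is a clickable cube actor that intensifies its material with each click.
; BeginPlay creates a dynamic material instance on the Cube component.
; Each click multiplies Scala by Offset, writes it to the "Intensity" parameter, and plays a click sound at a steadily falling pitch.
; The final threshold check on Scala has no effect, and the DestroyActor node is disconnected.
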(event OnClicked(Cube)
  (params (TouchedComponent :type Primitive%20Component%20Object%20Reference) (ButtonPressed :type Key%20Structure :default "None"))
  (bind _output_get (Variables|Default|SetScala (* (Variables|Default|GetScala) (Variables|Default|GetOffset))))
  (Rendering|Material|SetScalarParameterValue (Variables|Default|GetMaterial%20Instance) "Intensity" _output_get :!class /Script/Engine.MaterialInstanceDynamic)
  (Audio|PlaySound2D "/Engine/VREditor/Sounds/UI/Click_on_Button.Click_on_Button" 1.0 (Variables|Default|GetSoundPitch) 0.0 0 0)
  (Variables|Default|SetSoundPitch (- (Variables|Default|GetSoundPitch) 0.02))
  (if (> _output_get 1e+04)
    _))

(event EventBeginPlay
  (bind _returnvalue (Rendering|Material|CreateDynamicMaterialInstance (Variables|Default|GetCube) 0 0 "None" :!class /Script/Engine.PrimitiveComponent))
  (Variables|Default|SetMaterial%20Instance _returnvalue))

(event Collision|EventActorBeginOverlap
  (params (OtherActor :type Actor%20Object%20Reference)))

(event EventTick
  (params (DeltaSeconds :type Float%20%28single-precision%29)))

(fn ConstructionScript)