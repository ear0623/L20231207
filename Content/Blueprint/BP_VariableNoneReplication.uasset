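; Demo actor, named for a non-replicated variable case, that displays a health value on a text render in a networked game.
; On BeginPlay, only the authority initializes health and starts a looping timer that calls UpdateHealth.
; UpdateHealth subtracts MaxHealth rather than a smaller step, resetting to max when health reaches zero or below.
; Tick writes the local health value to the text on every instance.
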(event EventBeginPlay
  (Networking|SwitchHasAuthority
    (:Authority
      (CallFunction|InitalizeHealth)
      (Utilities|Time|SetTimerbyFunctionName 0 "UpdateHealth" (Variables|Default|GetHealthDecrementTime) true))))

(event Collision|EventActorBeginOverlap
  (params (OtherActor :type Actor%20Object%20Reference)))

(event EventTick
  (params (DeltaSeconds :type Float%20%28single-precision%29))
  (bind _textrender (Variables|Default|GetTextRender))
  (Utilities|IsValid _textrender
    (:Is%20Valid
      (Rendering|Components|TextRender|SetText _textrender (Utilities|Text|ToText(String) (Utilities|String|Append "Heath :" (Utilities|String|ToString(Integer) (Variables|Default|GetHeath))))))))

(fn ConstructionScript)

(fn UpdateHealth
  (bind _output_get (Variables|Default|SetHeath (- (Variables|Default|GetHeath) (Variables|Default|GetMaxHealth))))
  (if (<= _output_get 0)
    (CallFunction|InitalizeHealth)))

(fn InitalizeHealth
  (Variables|Default|SetHeath (Variables|Default|GetMaxHealth)))